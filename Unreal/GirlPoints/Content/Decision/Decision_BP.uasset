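; Decision point actor that prompts the player with a decision UI and removes itself when its trace is blocked.
; On overlap, it asks a Character_BP that is not moving to add the decision UI to the screen.
; Each tick, a Visibility line trace runs between its Start and End components.
; A hit sinks the actor with a latent move, then destroys it after a delay.
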(event `self.ReceiveActorBeginOverlap`
  (params (OtherActor :type "Actor Object Reference"))
  (bind _ascharacter_bp (cast `/Game/Character/Character_BP` OtherActor))
  (if (not (`/Game/Character/Character_BP.IsMoving` _ascharacter_bp))
    (`/Game/Character/Character_BP.AddDecisionUIToScreen` _ascharacter_bp)))

(event `self.ReceiveTick`
  (params (DeltaSeconds :type "Float (single-precision)"))
  ;[1 1 1] MoveToCharacter
  (bind (_outhit _returnvalue) (`KismetSystemLibrary.LineTraceSingle` (`SceneComponent.K2_GetComponentLocation` (`self.Start`)) (`SceneComponent.K2_GetComponentLocation` (`self.End`)) "TraceTypeQuery1"))
  (if _returnvalue
    (`KismetSystemLibrary.MoveComponentTo` (`self.K2_GetRootComponent`) (+ (`self.K2_GetActorLocation`) (0.0 0.0 -100.0)) (struct) false false 2.0)
    (`KismetSystemLibrary.Delay` 2.0)
    (`self.K2_DestroyActor`)))

(fn `UserConstructionScript`)