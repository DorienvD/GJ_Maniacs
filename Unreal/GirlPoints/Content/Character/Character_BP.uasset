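; Player character for a dice-driven board game that rolls Dice_BP on left click and advances one step per pip.
; Line traces to EndX and EndY choose each eased MoveComponentTo step, favouring X and switching to Y when blocked.
; Hardcoded per-value Delay chains call MovementCheck with input disabled, though one roll-of-five branch never re-enables it.
; BeginPlay adds the UI widget, while the intro dialogue logic is disconnected.
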(event `Key|LeftMouseButton`
  (params (Key :type "Key Structure" :default "AnyKey"))
  (bind _returnvalue (`GameplayStatics.GetPlayerCharacter` 0))
  (bind _returnvalue_2 (`GameplayStatics.GetPlayerCharacter` 0))
  (bind _returnvalue_3 (`GameplayStatics.GetPlayerCharacter` 0))
  (bind _returnvalue_4 (`GameplayStatics.GetPlayerCharacter` 0))
  (bind _returnvalue_5 (`GameplayStatics.GetPlayerCharacter` 0))
  (bind _returnvalue_6 (`GameplayStatics.GetPlayerCharacter` 0))
  (bind _returnvalue_7 (`GameplayStatics.GetPlayerCharacter` 0))
  (bind _returnvalue_8 (`GameplayStatics.GetPlayerCharacter` 0))
  (bind _returnvalue_9 (`GameplayStatics.GetPlayerCharacter` 0))
  (bind _returnvalue_10 (`GameplayStatics.GetPlayerCharacter` 0))
  (bind _returnvalue_11 (`GameplayStatics.GetPlayerCharacter` 0))
  (bind _returnvalue_12 (`GameplayStatics.GetPlayerCharacter` 0))
  (bind _returnvalue_13 (`GameplayStatics.GetPlayerCharacter` 0))
  (bind _returnvalue_14 (`GameplayStatics.GetPlayerCharacter` 0))
  (bind _returnvalue_15 (`GameplayStatics.GetPlayerCharacter` 0))
  (bind _returnvalue_16 (`GameplayStatics.GetPlayerCharacter` 0))
  (bind _returnvalue_17 (`GameplayStatics.GetPlayerCharacter` 0))
  (bind _returnvalue_18 (`GameplayStatics.GetPlayerCharacter` 0))
  ;[1 1 1] DiceMovement
  (:`Pressed`
    (set `self.IsMoving` true)
    (`self.DisableInput` null)
    (bind _outactors (`GameplayStatics.GetAllActorsOfClass` "/Game/Dice/Dice_BP.Dice_BP_C"))
    (for _array_element _outactors
      (bind _asdice_bp (cast `/Game/Dice/Dice_BP` _array_element))
      (`/Game/Dice/Dice_BP.DiceRoll` _asdice_bp)
      (bind (_outhit _returnvalue_19) (`KismetSystemLibrary.LineTraceSingle` (`SceneComponent.K2_GetComponentLocation` (`self.Start`)) (`SceneComponent.K2_GetComponentLocation` (`self.EndX`)) "TraceTypeQuery1"))
      (if _returnvalue_19
        (if (`self.MovedIn-Y`)
          (`|ExecutionSequence` :!label _label
            (:`then_0`
              (bind _dicevalue (`/Game/Dice/Dice_BP.DiceValue` _asdice_bp))
              (bind _returnvalue_20 (== _dicevalue 1))
              (if _returnvalue_20
                (set `self.MovedIn-Y` true)
                (`KismetSystemLibrary.MoveComponentTo` (`self.K2_GetRootComponent` _returnvalue_14) (+ (`self.K2_GetActorLocation` _returnvalue_14) (`self.MoveDistance-Y`)) (struct) true true 1.0)
                (`KismetSystemLibrary.Delay` 1.0)
                (`self.EnableInput` null)))
            (:`then_1`
              (bind _returnvalue_21 (== _dicevalue 2))
              (if _returnvalue_21
                (set `self.MovedIn-Y` true)
                (`KismetSystemLibrary.MoveComponentTo` (`self.K2_GetRootComponent` _returnvalue_15) (+ (`self.K2_GetActorLocation` _returnvalue_15) (`self.MoveDistance-Y`)) (struct) true true 1.0)
                (`KismetSystemLibrary.Delay` 0.2)
                (`self.MovementCheck`)
                (`KismetSystemLibrary.Delay` 1.0)
                (`self.EnableInput` null)))
            (:`then_2`
              (bind _returnvalue_22 (== _dicevalue 3))
              (if _returnvalue_22
                (set `self.MovedIn-Y` true)
                (`KismetSystemLibrary.MoveComponentTo` (`self.K2_GetRootComponent` _returnvalue_16) (+ (`self.K2_GetActorLocation` _returnvalue_16) (`self.MoveDistance-Y`)) (struct) true true 1.0)
                (`KismetSystemLibrary.Delay` 0.2)
                (`self.MovementCheck`)
                (`KismetSystemLibrary.Delay` 1.0)
                (`self.MovementCheck`)
                (`KismetSystemLibrary.Delay` 1.0)
                (`self.EnableInput` null)))
            (:`then_3`
              (bind _returnvalue_23 (== _dicevalue 4))
              (if _returnvalue_23
                (set `self.MovedIn-Y` true)
                (`KismetSystemLibrary.MoveComponentTo` (`self.K2_GetRootComponent` _returnvalue_17) (+ (`self.K2_GetActorLocation` _returnvalue_17) (`self.MoveDistance-Y`)) (struct) true true 1.0)
                (`KismetSystemLibrary.Delay` 0.2)
                (`self.MovementCheck`)
                (`KismetSystemLibrary.Delay` 1.0)
                (`self.MovementCheck`)
                (`KismetSystemLibrary.Delay` 1.0)
                (`self.MovementCheck`)
                (`KismetSystemLibrary.Delay` 1.0)
                (`self.EnableInput` null)))
            (:`then_4`
              (bind _returnvalue_24 (== _dicevalue 5))
              (if _returnvalue_24
                (set `self.MovedIn-Y` true)
                (`KismetSystemLibrary.MoveComponentTo` (`self.K2_GetRootComponent` _returnvalue_18) (+ (`self.K2_GetActorLocation` _returnvalue_18) (`self.MoveDistance-Y`)) (struct) true true 1.0)
                (`KismetSystemLibrary.Delay` 0.2)
                (`self.MovementCheck`)
                (`KismetSystemLibrary.Delay` 1.0)
                (`self.MovementCheck`)
                (`KismetSystemLibrary.Delay` 1.0)
                (`self.MovementCheck`)
                (`KismetSystemLibrary.Delay` 1.0)
                (`self.MovementCheck`)
                (`KismetSystemLibrary.Delay` 1.0)
                (`self.EnableInput` null)))
            (:`then_5`
              (bind _returnvalue_25 (== _dicevalue 6))
              (if _returnvalue_25
                (set `self.MovedIn-Y` true)
                (`KismetSystemLibrary.MoveComponentTo` (`self.K2_GetRootComponent` _returnvalue_13) (+ (`self.K2_GetActorLocation` _returnvalue_13) (`self.MoveDistance-Y`)) (struct) true true 1.0)
                (`KismetSystemLibrary.Delay` 0.2)
                (`self.MovementCheck`)
                (`KismetSystemLibrary.Delay` 1.0)
                (`self.MovementCheck`)
                (`KismetSystemLibrary.Delay` 1.0)
                (`self.MovementCheck`)
                (`KismetSystemLibrary.Delay` 1.0)
                (`self.MovementCheck`)
                (`KismetSystemLibrary.Delay` 1.0)
                (`self.MovementCheck`)
                (`KismetSystemLibrary.Delay` 1.0)
                (`self.EnableInput` null))))
          (else
            (bind (_outhit_2 _returnvalue_26) (`KismetSystemLibrary.LineTraceSingle` (`SceneComponent.K2_GetComponentLocation` (`self.Start`)) (`SceneComponent.K2_GetComponentLocation` (`self.EndY`)) "TraceTypeQuery1"))
            (if _returnvalue_26
              (`KismetSystemLibrary.LineTraceSingle` (`SceneComponent.K2_GetComponentLocation` (`self.Start`)) (`SceneComponent.K2_GetComponentLocation` (`self.End-Y`)) "TraceTypeQuery1")
              (goto _label)
              (else
                (`|ExecutionSequence`
                  (:`then_0`
                    (if _returnvalue_20
                      (`KismetSystemLibrary.MoveComponentTo` (`self.K2_GetRootComponent` _returnvalue_6) (+ (`self.K2_GetActorLocation` _returnvalue_6) (`self.MoveDistanceY`)) (struct) true true 1.0)
                      (`KismetSystemLibrary.Delay` 1.0)
                      (`self.EnableInput` null)))
                  (:`then_1`
                    (if _returnvalue_21
                      (`KismetSystemLibrary.MoveComponentTo` (`self.K2_GetRootComponent` _returnvalue_7) (+ (`self.K2_GetActorLocation` _returnvalue_7) (`self.MoveDistanceY`)) (struct) true true 1.0)
                      (`KismetSystemLibrary.Delay` 0.2)
                      (`self.MovementCheck`)
                      (`KismetSystemLibrary.Delay` 1.0)
                      (`self.EnableInput` null)))
                  (:`then_2`
                    (if _returnvalue_22
                      (`KismetSystemLibrary.MoveComponentTo` (`self.K2_GetRootComponent` _returnvalue_8) (+ (`self.K2_GetActorLocation` _returnvalue_8) (`self.MoveDistanceY`)) (struct) true true 1.0)
                      (`KismetSystemLibrary.Delay` 0.2)
                      (`self.MovementCheck`)
                      (`KismetSystemLibrary.Delay` 1.0)
                      (`self.MovementCheck`)
                      (`KismetSystemLibrary.Delay` 1.0)
                      (`self.EnableInput` null)))
                  (:`then_3`
                    (if _returnvalue_23
                      (`KismetSystemLibrary.MoveComponentTo` (`self.K2_GetRootComponent` _returnvalue_9) (+ (`self.K2_GetActorLocation` _returnvalue_9) (`self.MoveDistanceY`)) (struct) true true 1.0)
                      (`KismetSystemLibrary.Delay` 0.2)
                      (`self.MovementCheck`)
                      (`KismetSystemLibrary.Delay` 1.0)
                      (`self.MovementCheck`)
                      (`KismetSystemLibrary.Delay` 1.0)
                      (`self.MovementCheck`)
                      (`KismetSystemLibrary.Delay` 1.0)
                      (`self.EnableInput` null)))
                  (:`then_4`
                    (if _returnvalue_24
                      (`KismetSystemLibrary.MoveComponentTo` (`self.K2_GetRootComponent` _returnvalue_10) (+ (`self.K2_GetActorLocation` _returnvalue_10) (`self.MoveDistanceY`)) (struct) true true 1.0)
                      (`KismetSystemLibrary.Delay` 0.2)))
                  (:`then_5`
                    (if _returnvalue_25
                      (`KismetSystemLibrary.MoveComponentTo` (`self.K2_GetRootComponent` _returnvalue_11) (+ (`self.K2_GetActorLocation` _returnvalue_11) (`self.MoveDistanceY`)) (struct) true true 1.0)
                      (`KismetSystemLibrary.Delay` 0.2)
                      (`self.MovementCheck`)
                      (`KismetSystemLibrary.Delay` 1.0)
                      (`self.MovementCheck`)
                      (`KismetSystemLibrary.Delay` 1.0)
                      (`self.MovementCheck`)
                      (`KismetSystemLibrary.Delay` 1.0)
                      (`self.MovementCheck`)
                      (`KismetSystemLibrary.Delay` 1.0)
                      (`self.MovementCheck`)
                      (`KismetSystemLibrary.Delay` 1.0)
                      (`self.EnableInput` null))))))))
        (else
          (`|ExecutionSequence`
            (:`then_0`
              (if _returnvalue_20
                (`KismetSystemLibrary.MoveComponentTo` (`self.K2_GetRootComponent` _returnvalue) (+ (`self.K2_GetActorLocation` _returnvalue) (`self.MoveDistanceX`)) (struct) true true 1.0)
                (`KismetSystemLibrary.Delay` 1.0)
                (`self.EnableInput` null)))
            (:`then_1`
              (if _returnvalue_21
                (`KismetSystemLibrary.MoveComponentTo` (`self.K2_GetRootComponent` _returnvalue_12) (+ (`self.K2_GetActorLocation` _returnvalue_12) (`self.MoveDistanceX`)) (struct) true true 1.0)
                (`KismetSystemLibrary.Delay` 0.2)
                (`self.MovementCheck`)
                (`KismetSystemLibrary.Delay` 1.0)
                (`self.EnableInput` null)))
            (:`then_2`
              (if _returnvalue_22
                (`KismetSystemLibrary.MoveComponentTo` (`self.K2_GetRootComponent` _returnvalue_2) (+ (`self.K2_GetActorLocation` _returnvalue_2) (`self.MoveDistanceX`)) (struct) true true 1.0)
                (`KismetSystemLibrary.Delay` 0.2)
                (`self.MovementCheck`)
                (`KismetSystemLibrary.Delay` 1.0)
                (`self.MovementCheck`)
                (`KismetSystemLibrary.Delay` 1.0)
                (`self.EnableInput` null)))
            (:`then_3`
              (if _returnvalue_23
                (`KismetSystemLibrary.MoveComponentTo` (`self.K2_GetRootComponent` _returnvalue_3) (+ (`self.K2_GetActorLocation` _returnvalue_3) (`self.MoveDistanceX`)) (struct) true true 1.0)
                (`KismetSystemLibrary.Delay` 0.2)
                (`self.MovementCheck`)
                (`KismetSystemLibrary.Delay` 1.0)
                (`self.MovementCheck`)
                (`KismetSystemLibrary.Delay` 1.0)
                (`self.MovementCheck`)
                (`KismetSystemLibrary.Delay` 1.0)
                (`self.EnableInput` null)))
            (:`then_4`
              (if _returnvalue_24
                (`KismetSystemLibrary.MoveComponentTo` (`self.K2_GetRootComponent` _returnvalue_4) (+ (`self.K2_GetActorLocation` _returnvalue_4) (`self.MoveDistanceX`)) (struct) true true 1.0)
                (`KismetSystemLibrary.Delay` 0.2)
                (`self.MovementCheck`)
                (`KismetSystemLibrary.Delay` 1.0)
                (`self.MovementCheck`)
                (`KismetSystemLibrary.Delay` 1.0)
                (`self.MovementCheck`)
                (`KismetSystemLibrary.Delay` 1.0)
                (`self.MovementCheck`)
                (`KismetSystemLibrary.Delay` 1.0)
                (`self.EnableInput` null)))
            (:`then_5`
              (if _returnvalue_25
                (`KismetSystemLibrary.MoveComponentTo` (`self.K2_GetRootComponent` _returnvalue_5) (+ (`self.K2_GetActorLocation` _returnvalue_5) (`self.MoveDistanceX`)) (struct) true true 1.0)
                (`KismetSystemLibrary.Delay` 0.2)
                (`self.MovementCheck`)
                (`KismetSystemLibrary.Delay` 1.0)
                (`self.MovementCheck`)
                (`KismetSystemLibrary.Delay` 1.0)
                (`self.MovementCheck`)
                (`KismetSystemLibrary.Delay` 1.0)
                (`self.MovementCheck`)
                (`KismetSystemLibrary.Delay` 1.0)
                (`self.MovementCheck`)
                (`KismetSystemLibrary.Delay` 1.0)
                (`self.EnableInput` null)))))))))

(event `self.ReceiveBeginPlay`
  ;[1 1 1] IntroDialogue
  ;[1 1 1] ViewUI
  (bind _returnvalue (`|CreateWidget` "/Game/UI/UI_Widget.UI_Widget_C" :!label _label_2))
  (`UserWidget.AddToViewport` _returnvalue 0))

(event `AddUIToScreen`
  ;[1 1 1] ViewUI
  (goto _label_2))

(event `MovementCheck`
  (bind _returnvalue (`GameplayStatics.GetPlayerCharacter` 0))
  (bind _returnvalue_2 (`GameplayStatics.GetPlayerCharacter` 0))
  (bind _returnvalue_3 (`GameplayStatics.GetPlayerCharacter` 0))
  (bind _returnvalue_4 (`GameplayStatics.GetPlayerCharacter` 0))
  ;[1 1 1] MovementCheck
  (set `self.IsMoving` true)
  (bind (_outhit _returnvalue_5) (`KismetSystemLibrary.LineTraceSingle` (`SceneComponent.K2_GetComponentLocation` (`self.Start`)) (`SceneComponent.K2_GetComponentLocation` (`self.EndX`)) "TraceTypeQuery1"))
  (if _returnvalue_5
    (if (`self.MovedIn-Y`)
      (bind (_outhit_2 _returnvalue_6) (`KismetSystemLibrary.LineTraceSingle` (`SceneComponent.K2_GetComponentLocation` (`self.Start`)) (`SceneComponent.K2_GetComponentLocation` (`self.End-Y`)) "TraceTypeQuery1" :!label _label_3))
      (if _returnvalue_6
        (bind (_outhit_3 _returnvalue_7) (`KismetSystemLibrary.LineTraceSingle` (`SceneComponent.K2_GetComponentLocation` (`self.Start`)) (`SceneComponent.K2_GetComponentLocation` (`self.EndX`)) "TraceTypeQuery1"))
        (if (not _returnvalue_7)
          (`KismetSystemLibrary.MoveComponentTo` (`self.K2_GetRootComponent` _returnvalue) (+ (`self.K2_GetActorLocation` _returnvalue) (`self.MoveDistanceX`)) (struct) true true 1.0))
        (else
          (set `self.MovedIn-Y` true)
          (`KismetSystemLibrary.MoveComponentTo` (`self.K2_GetRootComponent` _returnvalue_3) (+ (`self.K2_GetActorLocation` _returnvalue_3) (`self.MoveDistance-Y`)) (struct) true true 1.0)))
      (else
        (bind (_outhit_4 _returnvalue_8) (`KismetSystemLibrary.LineTraceSingle` (`SceneComponent.K2_GetComponentLocation` (`self.Start`)) (`SceneComponent.K2_GetComponentLocation` (`self.EndY`)) "TraceTypeQuery1"))
        (if _returnvalue_8
          (goto _label_3)
          (else
            (`KismetSystemLibrary.MoveComponentTo` (`self.K2_GetRootComponent` _returnvalue_2) (+ (`self.K2_GetActorLocation` _returnvalue_2) (`self.MoveDistanceY`)) (struct) true true 1.0)))))
    (else
      (`KismetSystemLibrary.MoveComponentTo` (`self.K2_GetRootComponent` _returnvalue_4) (+ (`self.K2_GetActorLocation` _returnvalue_4) (`self.MoveDistanceX`)) (struct) true true 1.0))))

(fn `UserConstructionScript`)